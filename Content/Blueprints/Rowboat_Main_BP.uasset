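; Rowboat actor that keeps the player's BP_MotionCharacter seated in it.
; BeginPlay caches the player pawn and, after a zero-second delay, records the starting control rotation and sets IsSpawned.
; Every Tick snaps the character to SeatPosition and turns it to the boat's forward vector.
; Its CameraBasic takes controller pitch and yaw relative to the starting yaw, allowing free look while the body follows the boat.
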(event EventBeginPlay
  (bind _asbp_motion_character (Utilities|Casting|CastToBP_MotionCharacter (Game|Player|GetPlayerPawn 0)))
  (Variables|Default|SetMotionCharacterReference _asbp_motion_character)
  (Utilities|FlowControl|Delay 0.0)
  (Variables|Default|SetInitialControllerRotation (Pawn|GetControlRotation (Game|GetPlayerController 0) :!class /Script/Engine.Controller))
  (Variables|Default|SetIsSpawned? true))

(event Collision|EventActorBeginOverlap
  (params (OtherActor :type Actor%20Object%20Reference)))

(event EventTick
  (params (DeltaSeconds :type Float%20%28single-precision%29))
  (bind _returnvalue (Game|GetPlayerController 0))
  (bind _motioncharacterreference (Variables|Default|GetMotionCharacterReference))
  (bind _returnvalue_2 (Pawn|GetControlRotation _returnvalue :!class /Script/Engine.Controller))
  (bind (_roll _pitch _yaw) (Math|Rotator|BreakRotator _returnvalue_2))
  (Transformation|SetActorLocation (Variables|Default|GetMotionCharacterReference) (Transformation|GetWorldLocation (Variables|Default|GetSeatPosition)) false false)
  (Transformation|SetRelativeRotation (Variables|/Game/Blueprints/BP_MotionCharacter.BP_MotionCharacter_C|GetCamera_Basic _motioncharacterreference) (Math|Rotator|MakeRotator 0.0 _pitch (- _yaw (.Yaw (Math|Rotator|BreakRotator (Variables|Default|GetInitialControllerRotation))))) false false)
  (Transformation|SetActorRotation _motioncharacterreference (Math|Conversions|RotationFromXVector (Transformation|GetActorForwardVector self))))

(fn ConstructionScript)