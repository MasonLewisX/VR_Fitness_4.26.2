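; Blueprint that receives pedal and wheel sensor signals over UDP to propel the bicycle character.
; Each JSON packet's Pedal and Wheel booleans drive DoOnce gates that time the interval between pulses.
; Wheel pulses derive speed from circumference and interval, then launch Bicycle_Main_BP along its DirectionVector; pedal pulses also overwrite AddedSpeed, using the wheel interval.
; Tick prints debug values; an older count-based RPM, distance and km/h calculation is left disconnected.
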(event OnReceivedBytes(UDP)
  (params (Bytes :type Array%20of%20Bytes))
  (bind _returnvalue (Utilities|Time|GetGameTimeinSeconds))
  (bind _bicycle_main_bp (Variables|Default|GetBicycle_Main_BP))
  (bind _directionvector (Variables|/Game/Blueprints/Bicycle_Main_BP.Bicycle_Main_BP_C|GetDirectionVector _bicycle_main_bp))
  (bind (_x _y _z) (Math|Vector|BreakVector _directionvector))
  (bind _returnvalue_2 (Class|SIOJsonValue|AsObject (Class|SIOJsonValue|ValuefromJsonString (Class|CUBlueprintLibrary|ToString(Bytes) Bytes))))
  (Utilities|FlowControl|Sequence
    (:then_0
      (if (not (Class|SIOJsonObject|GetBoolField _returnvalue_2 "Pedal")) ; Signal Pedal On?
        (if (Variables|Default|GetIsPedalPassed?)
          (goto _label Reset))
        (else
          (Utilities|FlowControl|DoOnce false :!label _label
            (:Completed
              (Utilities|FlowControl|Sequence
                (:then_0
                  (Development|PrintString "Hello"))
                (:then_1
                  (Variables|Default|SetIsPedalPassed? false)
                  (bind _output_get (Variables|Default|SetNewPedalTime _returnvalue))
                  (Variables|Default|SetDeltaTimePedal (- _output_get (Variables|Default|GetPreviousPedalTime)))
                  (Variables|Default|SetPreviousPedalTime (Variables|Default|GetNewPedalTime))
                  (Variables|Default|SetIsPedalPassed? false)
                  (Variables|Default|SetIsPedalInitial? false)
                  (Variables|Default|SetAddedSpeed (/ (/ (* (Math|Float|MultiplybyPi 2.0) (Variables|Default|GetPedalRadius)) 1e+01) (Variables|Default|GetDeltaWheelTime))))))))))
    (:then_1
      (if (not (Class|SIOJsonObject|GetBoolField _returnvalue_2 "Wheel")) ; Signal Wheel On?
        (bind _output_get_2 (Variables|Default|SetIsWheelPassed? true))
        (Utilities|FlowControl|DoOnce false :!label _label_2
          (:Completed
            (Variables|Default|SetIsWheelPassed? false)
            (bind _output_get_3 (Variables|Default|SetNewWheelTime _returnvalue))
            (Variables|Default|SetDeltaWheelTime (- _output_get_3 (Variables|Default|GetPreviousWheelTime)))
            (Variables|Default|SetPreviousWheelTime (Variables|Default|GetNewWheelTime))
            (Variables|Default|SetIsWheelPassed? false)
            (Variables|Default|SetIsWheelInitial? false)
            (if (not (Variables|Default|GetIsWheelInitial?))
              ;[1 1 1] Additional Bicycle Speed
              (Variables|Default|SetAddedSpeed (/ (/ (* (Math|Float|MultiplybyPi 2.0) (/ (/ (Variables|Default|GetWheelDiameter) 1e+01) 2.0)) 1e+01) (Variables|Default|GetDeltaWheelTime))) ; AddedSpeed(cm/s)
              (Character|LaunchCharacter (Variables|Default|GetBicycle_Main_BP) (Math|Vector|MakeVector (* _x (* (Variables|Default|GetAddedSpeed) 1e+02)) (* _y (* (Variables|Default|GetAddedSpeed) 1e+02)) _z) false false))))
        (elif (not (Variables|Default|GetIsWheelInitial?))
          (if _output_get_2
            (goto _label_2 Reset)))))))

(event EventBeginPlay
  (bind _outactors (Actor|GetAllActorsOfClass "/Game/Blueprints/Bicycle_Main_BP.Bicycle_Main_BP_C"))
  (Variables|Default|SetBicycle_Main_BP (Utilities|Array|Get(acopy) _outactors)))

(event EventTick
  (params (DeltaSeconds :type Float%20%28single-precision%29))
  (Utilities|FlowControl|Sequence
    (:then_0
      (Development|PrintString (Utilities|String|ToString(Float) (Variables|Default|GetDeltaTimePedal)) true true "(R=1.000000,G=0.000000,B=0.000000,A=1.000000)" 0.002))
    (:then_2
      (Development|PrintString (Utilities|String|ToString(Float) (Variables|Default|GetDeltaWheelTime)) true true "(R=0.060894,G=1.000000,B=0.000000,A=1.000000)" 0.002))
    (:then_3
      (Development|PrintString (Utilities|String|ToString(Float) (Variables|Default|GetAddedSpeed)) true true "(R=1.000000,G=0.936362,B=0.000000,A=1.000000)" 0.002))
    (:then_4
      (Development|PrintString (Utilities|String|ToString(Boolean) (Variables|Default|GetIsClosed?)) true true "(R=1.000000,G=0.000000,B=0.000000,A=1.000000)" 0.002))))

(fn ConstructionScript)