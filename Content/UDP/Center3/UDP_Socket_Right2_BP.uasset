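; UDP socket Blueprint that receives rotation data for a second right-side source and stores it in UDPRight2Rotate.
; Received bytes are converted to a string, parsed as a JSON object and read for Pitch, Yaw and Roll.
; The axes are remapped: Pitch feeds X roll, Yaw feeds Y pitch and Roll feeds Z yaw.
; The nodes to start listening on port 3005 and close the socket never run here.
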(event OnReceivedBytes(UDP)
  (params (Bytes :type Array%20of%20Bytes))
  (bind _returnvalue (Class|SIOJsonValue|AsObject (Class|SIOJsonValue|ValuefromJsonString (Class|CUBlueprintLibrary|ToString(Bytes) Bytes))))
  (Variables|Default|SetUDP_Right2_Rotate (Math|Rotator|MakeRotator (Class|SIOJsonObject|GetNumberField _returnvalue "Pitch") (Class|SIOJsonObject|GetNumberField _returnvalue "Yaw") (Class|SIOJsonObject|GetNumberField _returnvalue "Roll"))))

(fn ConstructionScript)