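; UDP socket Blueprint that receives orientation data, labelled as Arduino quaternion, for "Center3" and stores it as the UDPCenter3Rotate rotator.
; Received bytes are parsed as JSON, and the qx, qy, qz, qw fields become a rotator.
; Axes are swapped and negated, with fixed offsets to align the gyro's zero.
; Calls to start listening on port 3003 and close the socket are unwired, so never run here.
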(event OnReceivedBytes(UDP)
  (params (Bytes :type Array%20of%20Bytes))
  (bind _returnvalue (Class|SIOJsonValue|AsObject (Class|SIOJsonValue|ValuefromJsonString (Class|CUBlueprintLibrary|ToString(Bytes) Bytes))))
  (Variables|Default|SetUDP_Center3_Rotate (Math|Rotator|MakeRotator (- (.Roll (Math|Rotator|BreakRotator (Math|Rotator|MakeRotator (.Roll (Math|Rotator|BreakRotator (Class|KismetMathLibrary|QuatRotator (Utilities|Struct|MakeQuat (Class|SIOJsonObject|GetNumberField _returnvalue "qx") (Class|SIOJsonObject|GetNumberField _returnvalue "qy") (Class|SIOJsonObject|GetNumberField _returnvalue "qz") (Class|SIOJsonObject|GetNumberField _returnvalue "qw"))))) (.Yaw (Math|Rotator|BreakRotator (Class|KismetMathLibrary|QuatRotator (Utilities|Struct|MakeQuat (Class|SIOJsonObject|GetNumberField _returnvalue "qx") (Class|SIOJsonObject|GetNumberField _returnvalue "qy") (Class|SIOJsonObject|GetNumberField _returnvalue "qz") (Class|SIOJsonObject|GetNumberField _returnvalue "qw"))))) (* (.Pitch (Math|Rotator|BreakRotator (Class|KismetMathLibrary|QuatRotator (Utilities|Struct|MakeQuat (Class|SIOJsonObject|GetNumberField _returnvalue "qx") (Class|SIOJsonObject|GetNumberField _returnvalue "qy") (Class|SIOJsonObject|GetNumberField _returnvalue "qz") (Class|SIOJsonObject|GetNumberField _returnvalue "qw"))))) -1.0)))) 96.0) (.Yaw (Math|Rotator|BreakRotator (Math|Rotator|MakeRotator (.Roll (Math|Rotator|BreakRotator (Class|KismetMathLibrary|QuatRotator (Utilities|Struct|MakeQuat (Class|SIOJsonObject|GetNumberField _returnvalue "qx") (Class|SIOJsonObject|GetNumberField _returnvalue "qy") (Class|SIOJsonObject|GetNumberField _returnvalue "qz") (Class|SIOJsonObject|GetNumberField _returnvalue "qw"))))) (.Yaw (Math|Rotator|BreakRotator (Class|KismetMathLibrary|QuatRotator (Utilities|Struct|MakeQuat (Class|SIOJsonObject|GetNumberField _returnvalue "qx") (Class|SIOJsonObject|GetNumberField _returnvalue "qy") (Class|SIOJsonObject|GetNumberField _returnvalue "qz") (Class|SIOJsonObject|GetNumberField _returnvalue "qw"))))) (* (.Pitch (Math|Rotator|BreakRotator (Class|KismetMathLibrary|QuatRotator (Utilities|Struct|MakeQuat (Class|SIOJsonObject|GetNumberField _returnvalue "qx") (Class|SIOJsonObject|GetNumberField _returnvalue "qy") (Class|SIOJsonObject|GetNumberField _returnvalue "qz") (Class|SIOJsonObject|GetNumberField _returnvalue "qw"))))) -1.0)))) (* (+ (.Pitch (Math|Rotator|BreakRotator (Math|Rotator|MakeRotator (.Roll (Math|Rotator|BreakRotator (Class|KismetMathLibrary|QuatRotator (Utilities|Struct|MakeQuat (Class|SIOJsonObject|GetNumberField _returnvalue "qx") (Class|SIOJsonObject|GetNumberField _returnvalue "qy") (Class|SIOJsonObject|GetNumberField _returnvalue "qz") (Class|SIOJsonObject|GetNumberField _returnvalue "qw"))))) (.Yaw (Math|Rotator|BreakRotator (Class|KismetMathLibrary|QuatRotator (Utilities|Struct|MakeQuat (Class|SIOJsonObject|GetNumberField _returnvalue "qx") (Class|SIOJsonObject|GetNumberField _returnvalue "qy") (Class|SIOJsonObject|GetNumberField _returnvalue "qz") (Class|SIOJsonObject|GetNumberField _returnvalue "qw"))))) (* (.Pitch (Math|Rotator|BreakRotator (Class|KismetMathLibrary|QuatRotator (Utilities|Struct|MakeQuat (Class|SIOJsonObject|GetNumberField _returnvalue "qx") (Class|SIOJsonObject|GetNumberField _returnvalue "qy") (Class|SIOJsonObject|GetNumberField _returnvalue "qz") (Class|SIOJsonObject|GetNumberField _returnvalue "qw"))))) -1.0)))) 1.2e+02) -1.0))))

(fn ConstructionScript)