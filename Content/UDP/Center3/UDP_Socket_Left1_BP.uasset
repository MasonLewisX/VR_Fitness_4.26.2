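; UDP socket Blueprint for the Left1 channel that turns received orientation packets into the UDPLeft1Rotate rotator.
; On each received packet it parses the bytes as JSON and converts the quaternion fields to a rotator.
; It swaps roll and pitch, negates all three axes, then adds fixed offsets to roll and yaw.
; The start-listening and close-socket calls are present but never run, so this graph does not open the socket itself.
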(event OnReceivedBytes(UDP)
  (params (Bytes :type Array%20of%20Bytes))
  (bind _returnvalue (Class|SIOJsonValue|AsObject (Class|SIOJsonValue|ValuefromJsonString (Class|CUBlueprintLibrary|ToString(Bytes) Bytes))))
  (Variables|Default|SetUDP_Left1_Rotate (Math|Rotator|MakeRotator (+ (.Roll (Math|Rotator|BreakRotator (Math|Rotator|MakeRotator (* (.Pitch (Math|Rotator|BreakRotator (Class|KismetMathLibrary|QuatRotator (Utilities|Struct|MakeQuat (Class|SIOJsonObject|GetNumberField _returnvalue "qx") (Class|SIOJsonObject|GetNumberField _returnvalue "qy") (Class|SIOJsonObject|GetNumberField _returnvalue "qz") (Class|SIOJsonObject|GetNumberField _returnvalue "qw"))))) -1.0) (* (.Roll (Math|Rotator|BreakRotator (Class|KismetMathLibrary|QuatRotator (Utilities|Struct|MakeQuat (Class|SIOJsonObject|GetNumberField _returnvalue "qx") (Class|SIOJsonObject|GetNumberField _returnvalue "qy") (Class|SIOJsonObject|GetNumberField _returnvalue "qz") (Class|SIOJsonObject|GetNumberField _returnvalue "qw"))))) -1.0) (* (.Yaw (Math|Rotator|BreakRotator (Class|KismetMathLibrary|QuatRotator (Utilities|Struct|MakeQuat (Class|SIOJsonObject|GetNumberField _returnvalue "qx") (Class|SIOJsonObject|GetNumberField _returnvalue "qy") (Class|SIOJsonObject|GetNumberField _returnvalue "qz") (Class|SIOJsonObject|GetNumberField _returnvalue "qw"))))) -1.0)))) 21.0) (.Pitch (Math|Rotator|BreakRotator (Math|Rotator|MakeRotator (* (.Pitch (Math|Rotator|BreakRotator (Class|KismetMathLibrary|QuatRotator (Utilities|Struct|MakeQuat (Class|SIOJsonObject|GetNumberField _returnvalue "qx") (Class|SIOJsonObject|GetNumberField _returnvalue "qy") (Class|SIOJsonObject|GetNumberField _returnvalue "qz") (Class|SIOJsonObject|GetNumberField _returnvalue "qw"))))) -1.0) (* (.Roll (Math|Rotator|BreakRotator (Class|KismetMathLibrary|QuatRotator (Utilities|Struct|MakeQuat (Class|SIOJsonObject|GetNumberField _returnvalue "qx") (Class|SIOJsonObject|GetNumberField _returnvalue "qy") (Class|SIOJsonObject|GetNumberField _returnvalue "qz") (Class|SIOJsonObject|GetNumberField _returnvalue "qw"))))) -1.0) (* (.Yaw (Math|Rotator|BreakRotator (Class|KismetMathLibrary|QuatRotator (Utilities|Struct|MakeQuat (Class|SIOJsonObject|GetNumberField _returnvalue "qx") (Class|SIOJsonObject|GetNumberField _returnvalue "qy") (Class|SIOJsonObject|GetNumberField _returnvalue "qz") (Class|SIOJsonObject|GetNumberField _returnvalue "qw"))))) -1.0)))) (- (.Yaw (Math|Rotator|BreakRotator (Math|Rotator|MakeRotator (* (.Pitch (Math|Rotator|BreakRotator (Class|KismetMathLibrary|QuatRotator (Utilities|Struct|MakeQuat (Class|SIOJsonObject|GetNumberField _returnvalue "qx") (Class|SIOJsonObject|GetNumberField _returnvalue "qy") (Class|SIOJsonObject|GetNumberField _returnvalue "qz") (Class|SIOJsonObject|GetNumberField _returnvalue "qw"))))) -1.0) (* (.Roll (Math|Rotator|BreakRotator (Class|KismetMathLibrary|QuatRotator (Utilities|Struct|MakeQuat (Class|SIOJsonObject|GetNumberField _returnvalue "qx") (Class|SIOJsonObject|GetNumberField _returnvalue "qy") (Class|SIOJsonObject|GetNumberField _returnvalue "qz") (Class|SIOJsonObject|GetNumberField _returnvalue "qw"))))) -1.0) (* (.Yaw (Math|Rotator|BreakRotator (Class|KismetMathLibrary|QuatRotator (Utilities|Struct|MakeQuat (Class|SIOJsonObject|GetNumberField _returnvalue "qx") (Class|SIOJsonObject|GetNumberField _returnvalue "qy") (Class|SIOJsonObject|GetNumberField _returnvalue "qz") (Class|SIOJsonObject|GetNumberField _returnvalue "qw"))))) -1.0)))) 84.0))))

(fn ConstructionScript)