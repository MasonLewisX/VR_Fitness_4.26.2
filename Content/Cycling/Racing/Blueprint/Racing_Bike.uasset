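; Player-controlled racing bicycle pawn built on vehicle movement, with steering, throttle, Shift sprint and a zoomable spring-arm camera with mouse orbit.
; Input axes drive the movement component, while timelines blend pose variables for steering, lean, idle and pedalling, apparently for animation.
; Sprint uses a gate opened on Tick during forward input, adding body sway and extra physics velocity.
; Throttle also toggles chain motion through a dynamic material.
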(event EventTick
  (params (DeltaSeconds :type Float%20%28single-precision%29))
  (bind _vehiclemovement (Variables|Default|GetVehicleMovement))
  ;[1 0.4217 0.3451] Sprint
  (Utilities|FlowControl|Sequence
    (:then_0
      ;[0.9302 1 0.5283] Idle
      (if (or (and (== (Input|AxisValues|GetMoveForward) 0.0) (< (Class|WheeledVehicleMovementComponent|GetEngineRotationSpeed _vehiclemovement) 2e+02)) (< (Class|WheeledVehicleMovementComponent|GetCurrentGear _vehiclemovement) 0))
        (bind _newtrack_0 (Timeline|Timeline_6 Play)
          (:Update
            (Variables|Default|SetIdle _newtrack_0)
            (Variables|Default|SetBody (Math|Rotator|Lerp(Rotator) (Variables|Default|GetBody) "0, 0,-10.000000" _newtrack_0))))
        (else
          (Timeline|Timeline_6 Reverse))))
    (:then_1
      (if (> (Input|AxisValues|GetMoveForward) 0.0)
        (Utilities|FlowControl|Gate true) ; enters at Open
        (else
          (bind _newtrack_0_2 (Timeline|Timeline_0 Stop)
            (:Update
              (Variables|Default|SetBody (Math|Rotator|MakeRotator _newtrack_0_2 0.0 0.0)))))))))

(event Input|AxisEvents|InputAxisLookRight
  (params (AxisValue :type Float%20%28single-precision%29))
  ;[0.4745 0.8144 1] Camera
  (Pawn|Input|AddControllerYawInput AxisValue))

(event Input|AxisEvents|InputAxisMoveForward
  (params (AxisValue :type Float%20%28single-precision%29))
  ;[0.8006 0.6394 1] MoveForward
  (Class|WheeledVehicleMovementComponent|SetThrottleInput (Variables|Default|GetVehicleMovement) AxisValue)
  (if (> AxisValue 0.1)
    (Variables|Default|SetSpeedRate 1.0)
    (Rendering|Material|SetScalarParameterValue (Variables|Default|GetChain) "Time" 1.0 :!class /Script/Engine.MaterialInstanceDynamic)
    (bind _newtrack_1 (Timeline|Timeline_7 PlayFromStart)
      (:Update
        (Variables|Default|SetBody (Math|Rotator|Lerp(Rotator) (Variables|Default|GetBody) "0, 0, 0" _newtrack_1))))
    (else
      (Variables|Default|SetSpeedRate 0.001)
      (Rendering|Material|SetScalarParameterValue (Variables|Default|GetChain) "Time" 0.0 :!class /Script/Engine.MaterialInstanceDynamic))))

(event Input|AxisEvents|InputAxisLookUp
  (params (AxisValue :type Float%20%28single-precision%29))
  ;[0.4745 0.8144 1] Camera
  (Pawn|Input|AddControllerPitchInput AxisValue))

(event Input|AxisEvents|InputAxisMoveRight
  (params (AxisValue :type Float%20%28single-precision%29))
  ;[0.8006 0.6394 1] MoveRight
  (Class|WheeledVehicleMovementComponent|SetSteeringInput (Variables|Default|GetVehicleMovement) AxisValue)
  (Utilities|FlowControl|Sequence
    (:then_0
      (if (> AxisValue 0.1)
        (bind _newtrack_2 (Timeline|Timeline_2 PlayFromStart)
          (:Update
            (Variables|Default|SetRot_F_Wheel (Math|Rotator|Lerp(Rotator) (Variables|Default|GetRot_F_Wheel) "0,10.000000,3.500000" _newtrack_2))
            (Variables|Default|SetHB (Math|Rotator|Lerp(Rotator) (Variables|Default|GetHB) "0, 0,10.000000" _newtrack_2))
            (Variables|Default|SetF_Wheel_V (Math|Vector|Lerp(Vector) (Variables|Default|GetF_Wheel_V) "0,0.500000, 0" _newtrack_2))
            (if (Variables|Default|GetShift)
              (Variables|Default|SetRight (Math|Float|Lerp (Variables|Default|GetRight) 0.4 _newtrack_2))
              (Variables|Default|SetLeft (Math|Float|Lerp (Variables|Default|GetLeft) 0.001 _newtrack_2))
              (Variables|Default|SetFast_Right (Math|Float|Lerp (Variables|Default|GetFast_Right) 0.001 _newtrack_2))
              (Variables|Default|SetFast_Left (Math|Float|Lerp (Variables|Default|GetFast_Left) 0.001 _newtrack_2))
              (else
                (Variables|Default|SetFast_Right (Math|Float|Lerp (Variables|Default|GetFast_Right) 0.5 _newtrack_2))
                (Variables|Default|SetFast_Left (Math|Float|Lerp (Variables|Default|GetFast_Left) 0.001 _newtrack_2))
                (Variables|Default|SetRight (Math|Float|Lerp (Variables|Default|GetRight) 0.001 _newtrack_2))
                (Variables|Default|SetLeft (Math|Float|Lerp (Variables|Default|GetLeft) 0.001 _newtrack_2))))))
        (else
          (Timeline|Timeline_2 Reverse))))
    (:then_1
      (if (< AxisValue -0.01)
        (bind _newtrack_2_2 (Timeline|Timeline_3 PlayFromStart)
          (:Update
            (Variables|Default|SetRot_F_Wheel (Math|Rotator|Lerp(Rotator) (Variables|Default|GetRot_F_Wheel) "0,-10.000000,-3.500000" _newtrack_2_2))
            (Variables|Default|SetHB (Math|Rotator|Lerp(Rotator) (Variables|Default|GetHB) "0, 0,-10.000000" _newtrack_2_2))
            (Variables|Default|SetF_Wheel_V (Math|Vector|Lerp(Vector) (Variables|Default|GetF_Wheel_V) "0,-0.500000, 0" _newtrack_2_2))
            (if (Variables|Default|GetShift)
              (Variables|Default|SetRight (Math|Float|Lerp (Variables|Default|GetRight) 0.001 _newtrack_2_2))
              (Variables|Default|SetLeft (Math|Float|Lerp (Variables|Default|GetLeft) 0.4 _newtrack_2_2))
              (Variables|Default|SetFast_Right (Math|Float|Lerp (Variables|Default|GetFast_Right) 0.001 _newtrack_2_2))
              (Variables|Default|SetFast_Left (Math|Float|Lerp (Variables|Default|GetFast_Left) 0.001 _newtrack_2_2))
              (else
                (Variables|Default|SetFast_Right (Math|Float|Lerp (Variables|Default|GetFast_Right) 0.001 _newtrack_2_2))
                (Variables|Default|SetFast_Left (Math|Float|Lerp (Variables|Default|GetFast_Left) 0.5 _newtrack_2_2))
                (Variables|Default|SetRight (Math|Float|Lerp (Variables|Default|GetRight) 0.001 _newtrack_2_2))
                (Variables|Default|SetLeft (Math|Float|Lerp (Variables|Default|GetLeft) 0.001 _newtrack_2_2))))))
        (else
          (Timeline|Timeline_3 Reverse))))
    (:then_2
      (if (== AxisValue 0.0)
        (bind _newtrack_2_3 (Timeline|Timeline_4 PlayFromStart)
          (:Update
            (Variables|Default|SetRot_F_Wheel (Math|Rotator|Lerp(Rotator) (Variables|Default|GetRot_F_Wheel) "0, 0, 0" _newtrack_2_3))
            (Variables|Default|SetHB (Math|Rotator|Lerp(Rotator) (Variables|Default|GetHB) "0, 0, 0" _newtrack_2_3))
            (Variables|Default|SetF_Wheel_V (Math|Vector|Lerp(Vector) (Variables|Default|GetF_Wheel_V) "0, 0, 0" _newtrack_2_3))
            (if (Variables|Default|GetShift)
              (Variables|Default|SetRight (Math|Float|Lerp (Variables|Default|GetRight) 0.001 _newtrack_2_3))
              (Variables|Default|SetLeft (Math|Float|Lerp (Variables|Default|GetLeft) 0.001 _newtrack_2_3))
              (Variables|Default|SetFast_Right (Math|Float|Lerp (Variables|Default|GetFast_Right) 0.001 _newtrack_2_3))
              (Variables|Default|SetFast_Left (Math|Float|Lerp (Variables|Default|GetFast_Left) 0.001 _newtrack_2_3))
              (else
                (Variables|Default|SetFast_Right (Math|Float|Lerp (Variables|Default|GetFast_Right) 0.001 _newtrack_2_3))
                (Variables|Default|SetFast_Left (Math|Float|Lerp (Variables|Default|GetFast_Left) 0.001 _newtrack_2_3))
                (Variables|Default|SetRight (Math|Float|Lerp (Variables|Default|GetRight) 0.001 _newtrack_2_3))
                (Variables|Default|SetLeft (Math|Float|Lerp (Variables|Default|GetLeft) 0.001 _newtrack_2_3))))))
        (else
          (Timeline|Timeline_4 Stop))))))

(event Input|KeyboardEvents|LeftShift
  (params (Key :type Key%20Structure :default "None"))
  ;[1 0.4217 0.3451] Sprint
  (:Pressed
    (Utilities|FlowControl|Gate true :!label _label
      (:Exit
        (Variables|Default|SetShift false)
        (Utilities|FlowControl|Sequence
          (:then_0
            (bind _newtrack_0 (Timeline|Timeline_1 PlayFromStart)
              (:Update
                (Variables|Default|SetFast (Math|Float|Lerp 0.001 1.0 _newtrack_0)))))
          (:then_1
            (bind _newtrack_0_2 (Timeline|Timeline_0 Play)
              (:Update
                (Variables|Default|SetBody (Math|Rotator|MakeRotator _newtrack_0_2 0.0 0.0)))))
          (:then_2
            (bind _newtrack_0_3 (Timeline|Timeline_5 PlayFromStart)
              (:Update
                (Physics|SetPhysicsLinearVelocity (Variables|Character|GetMesh) (Math|Vector|MakeVector (Math|Float|Lerp 0.0 (* (.X (Math|Vector|BreakVector (Math|Rotator|GetRotationXVector (Transformation|GetActorRotation)))) 3e+01) _newtrack_0_3) 0.0 0.0) true "root"))))))))
  (:Released
    (Utilities|FlowControl|Sequence
      (:then_0
        (goto _label Close))
      (:then_1
        (Variables|Default|SetShift true)
        (Utilities|FlowControl|Sequence
          (:then_0
            (Timeline|Timeline_0 Stop))
          (:then_1
            (Timeline|Timeline_1 Reverse))))
      (:then_2
        (Timeline|Timeline_5 Stop)))))

(event Input|MouseEvents|LeftMouseButton
  (params (Key :type Key%20Structure :default "None"))
  (bind _springarm (Variables|Default|GetSpringArm))
  ;[0.4745 0.8144 1] Camera
  (:Pressed
    (Variables|/Script/Engine.SpringArmComponent|SetbUsePawnControlRotation _springarm true))
  (:Released
    (Variables|/Script/Engine.SpringArmComponent|SetbUsePawnControlRotation _springarm false)))

(event Input|MouseEvents|RightMouseButton
  (params (Key :type Key%20Structure :default "None"))
  (bind _springarm (Variables|Default|GetSpringArm))
  ;[0.4745 0.8144 1] Camera
  (:Pressed
    (Variables|/Script/Engine.SpringArmComponent|SetbUsePawnControlRotation _springarm false)
    (Transformation|SetRelativeTransform _springarm (Math|Transform|MakeTransform "0, 0,47.476143" "-19.999990,39.999985, 0") false false)
    (Variables|/Script/Engine.SpringArmComponent|SetTargetArmLength _springarm 3e+02)))

(event Input|MouseEvents|MouseWheelUp
  (params (Key :type Key%20Structure :default "None"))
  ;[0.4745 0.8144 1] Camera
  (:Pressed
    (bind _newtrack_1 (Timeline|Timeline_8 Reverse)
      (:Update
        (Variables|/Script/Engine.SpringArmComponent|SetTargetArmLength (Variables|Default|GetSpringArm) (Math|Float|Lerp 3e+02 6e+02 _newtrack_1))))))

(event Input|MouseEvents|MouseWheelDown
  (params (Key :type Key%20Structure :default "None"))
  ;[0.4745 0.8144 1] Camera
  (:Pressed
    (bind _newtrack_1 (Timeline|Timeline_8 Play)
      (:Update
        (Variables|/Script/Engine.SpringArmComponent|SetTargetArmLength (Variables|Default|GetSpringArm) (Math|Float|Lerp 3e+02 6e+02 _newtrack_1))))))

(fn ConstructionScript
  (bind _returnvalue (Rendering|Material|CreateDynamicMaterialInstance (Variables|Default|GetChains) 0 "/Game/Cycling/Racing/Material/M_Chain_Inst.M_Chain_Inst" "None" :!class /Script/Engine.PrimitiveComponent))
  (Variables|Default|SetChain _returnvalue))